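; PCG editor tool that grows moss over a referenced static mesh actor and bakes it to a mesh asset.
; Construction fits the box to the target and feeds mesh, transform, scale-adjusted density and texture toggle to the PCG graph, optionally collecting per-material fuzz masks.
; Save sets a random-suffixed asset name and the graph's save flag.
; Place spawns that mesh attached to the target, then deactivates generation.
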(fn ConstructionScript
  (CallFunction|GenerateMoss))

(fn 01-SavetoAsset
  (bind _pcg (Variables|Default|GetPCG))
  (bind _graphinstance (Variables|/Script/PCG.PCGComponent|GetGraphInstance _pcg))
  (bind _name (CallFunction|GetRandomName 5))
  (Variables|BakeMesh|SetRandom%20Number _name)
  (Class|PCGGraphParametersHelpers|SetStringParameter _graphinstance "MeshPath" (Variables|BakeMesh|GetCustom%20Path))
  (Class|PCGGraphParametersHelpers|SetStringParameter _graphinstance "MeshName" (Utilities|String|Append (Variables|BakeMesh|GetCustom%20Name) "_" (Variables|BakeMesh|GetRandom%20Number)))
  (Variables|BakeMesh|SetMesh%20Name%20and%20Path (Utilities|String|Append (Variables|BakeMesh|GetCustom%20Path) (Utilities|String|Append (Variables|BakeMesh|GetCustom%20Name) "_" (Variables|BakeMesh|GetRandom%20Number)) "." (Utilities|String|Append (Variables|BakeMesh|GetCustom%20Name) "_" (Variables|BakeMesh|GetRandom%20Number))))
  (bind _asset_exists (CallFunction|ValidateAssetsExists (Variables|BakeMesh|GetMesh%20Name%20and%20Path)))
  (if (not _asset_exists)
    (Effects|Components|ParticleSystem|SetBoolParameter (Variables|/Script/PCG.PCGComponent|GetGraphInstance (Variables|Default|GetPCG)) "Savemesh" true)))

(fn 02-PlaceinLevel
  (bind _asset_exists (CallFunction|ValidateAssetsandPath (Variables|BakeMesh|GetMesh%20Name%20and%20Path)))
  (if _asset_exists
    (bind _returnvalue (Game|SpawnActorfromClass "/Game/Common/Tools/PCG/PCG_Moss/Blueprint/SM_PCGMoss.SM_PCGMoss_C" (Math|Conversions|ToTransform(Vector) (.location (Transformation|GetActorTransform))) "Undefined" "MultiplyWithRoot" 0 0))
    (bind _returnvalue_2 (Utilities|LoadAssetBlocking (Class|KismetSystemLibrary|ToSoftObjRef(SoftObjPath) (Utilities|MakeSoftObjectPath (Variables|BakeMesh|GetMesh%20Name%20and%20Path)))))
    (bind _asstatic_mesh (Utilities|Casting|CastToStaticMesh _returnvalue_2))
    (Components|StaticMesh|SetStaticMesh (Variables|/Script/Engine.StaticMeshActor|GetStaticMeshComponent _returnvalue) _asstatic_mesh)
    (Variables|/Script/Engine.ActorComponent|SetComponentTags (Variables|/Script/Engine.StaticMeshActor|GetStaticMeshComponent _returnvalue) (Utilities|Array|MakeArray "PCGMesh"))
    (Transformation|AttachActorToActor _returnvalue (Variables|01-Global|GetRerfenceMesh) "None" "KeepWorld" "KeepWorld" "KeepWorld" true)
    (Effects|Components|ParticleSystem|SetBoolParameter (Variables|/Script/PCG.PCGComponent|GetGraphInstance (Variables|Default|GetPCG)) "Savemesh" false)
    (Effects|Components|ParticleSystem|SetBoolParameter (Variables|/Script/PCG.PCGComponent|GetGraphInstance (Variables|Default|GetPCG)) "Active" false)
    (Variables|01-Global|SetActive false)
    (else
      (Development|PrintString "未生成资产，请重试！" true true "(R=1.000000,G=0.039770,B=0.009923,A=1.000000)" 1e+01))))

(fn ReGenerate
  (bind _pcg (Variables|Default|GetPCG))
  (Class|PCGComponent|CleanupLocal _pcg true false)
  (Class|PCGComponent|GenerateLocal _pcg true))

(fn ValidateAssetsandPath
  (params (Path :type String))
  (bind _returnvalue (Class|AssetRegistry|GetAssetbyObjectPath (Class|AssetRegistryHelpers|GetAssetRegistry) (Utilities|String|StringToName Path) false))
  (return (Utilities|IsValid (Class|AssetRegistryHelpers|GetAsset _returnvalue))))

(fn FuzzMask
  (Effects|Components|ParticleSystem|SetBoolParameter (Variables|/Script/PCG.PCGComponent|GetGraphInstance (Variables|Default|GetPCG)) "UseTexture" (Variables|03-Mask|GetUse%20Texture))
  (if (Variables|03-Mask|GetUse%20Texture)
    (if (Variables|03-Mask|GetFuzz%20Map%20From%20Material)
      (Utilities|Array|Clear (Variables|03-Mask|GetFuzz%20Map))
      (for _array_element (Rendering|Material|GetMaterials (Variables|/Script/Engine.StaticMeshActor|GetStaticMeshComponent (Variables|01-Global|GetRerfenceMesh)))
        (bind _asmaterial_instance_constant (Utilities|Casting|CastToMaterialInstanceConstant _array_element))
        (bind _returnvalue (Rendering|Material|GetTextureParameterValue _asmaterial_instance_constant "DRF" :!class /Script/Engine.MaterialInstanceConstant))
        (bind _returnvalue_2 (Rendering|Material|GetTextureParameterValue _asmaterial_instance_constant "FuzzMap" :!class /Script/Engine.MaterialInstanceConstant))
        (if (or (Utilities|IsValid _returnvalue_2) (and (Utilities|IsValid _returnvalue) (!= _returnvalue "/Game/Common/ShareAssets/Textures/T_Defalut_M.T_Defalut_M")))
          (Utilities|Array|Add (Variables|03-Mask|GetFuzz%20Map) (select (and (Utilities|IsValid _returnvalue) (!= _returnvalue "/Game/Common/ShareAssets/Textures/T_Defalut_M.T_Defalut_M")) _returnvalue _returnvalue_2))
          (else
            (Utilities|Array|Add (Variables|03-Mask|GetFuzz%20Map) "/Game/Common/ShareAssets/Textures/T_Defalut_D.T_Defalut_D")))))))

(fn SetBound
  (bind _rerfencemesh (Variables|01-Global|GetRerfenceMesh))
  (bind _box (Variables|Default|GetBox))
  (bind (_origin _boxextent) (Collision|GetActorBounds _rerfencemesh false false))
  (Transformation|SetWorldLocation _box _origin false false)
  (Components|Box|SetBoxExtent _box (Math|Vector|MakeVector (.x _boxextent) (.y _boxextent) (.z _boxextent)) true))

(fn GenerateMoss
  (bind _rerfencemesh (Variables|01-Global|GetRerfenceMesh))
  (bind _pcg (Variables|Default|GetPCG))
  (bind _pcg_2 (Variables|Default|GetPCG))
  (bind _pcg_3 (Variables|Default|GetPCG))
  (bind _rerfencemesh_2 (Variables|01-Global|GetRerfenceMesh))
  (bind _returnvalue (Transformation|GetActorTransform _rerfencemesh))
  (bind _graphinstance (Variables|/Script/PCG.PCGComponent|GetGraphInstance _pcg_3))
  (bind _graphinstance_2 (Variables|/Script/PCG.PCGComponent|GetGraphInstance _pcg))
  (bind _graphinstance_3 (Variables|/Script/PCG.PCGComponent|GetGraphInstance _pcg_2))
  (Utilities|IsValid _rerfencemesh
    (:Is%20Valid
      (Transformation|SetActorTransform self (Math|Transform|MakeTransform (.location _returnvalue) "0, 0, 0" "1.000000,1.000000,1.000000"))
      (CallFunction|SetBound))
    (:Is%20Not%20Valid
      _))
  (CallFunction|FuzzMask)
  (Effects|Components|ParticleSystem|SetFloatParameter _graphinstance_3 "CoverAmount" (/ (/ 1.0 (Variables|02-Fuzz|GetCover%20Density)) (Math|Vector|DotProduct (Math|Vector|VectorGetAbs (.scale _returnvalue)) "0.333000,0.333000,0.333000")))
  (Effects|Components|ParticleSystem|SetFloatParameter _graphinstance_3 "ObjectBoundScale" (/ (Math|Vector|DotProduct (.BoxExtent (Collision|GetActorBounds _rerfencemesh false false)) "0.333000,0.333000,0.333000") 4e+01))
  (Audio|Parameter|SetObjectParameter _graphinstance_2 "SelectMesh" (Variables|/Script/Engine.StaticMeshComponent|GetStaticMesh (Variables|/Script/Engine.StaticMeshActor|GetStaticMeshComponent _rerfencemesh_2)))
  (Class|PCGGraphParametersHelpers|SetTransformParameter _graphinstance_2 "MeshTransform" (Transformation|GetActorTransform _rerfencemesh_2))
  (if (Variables|01-Global|GetActive)
    (Effects|Components|ParticleSystem|SetBoolParameter _graphinstance "Active" true)
    (Variables|/Script/PCG.PCGComponent|SetbActivated _pcg_3 true)
    (else
      (Effects|Components|ParticleSystem|SetBoolParameter _graphinstance "Active" false)
      (Variables|/Script/PCG.PCGComponent|SetbActivated _pcg_3 false))))