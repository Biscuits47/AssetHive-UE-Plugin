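; BP_PCG_Fuzz is a custom PCG Blueprint element in the moss tool set that applies a material to a dynamic mesh.
; It casts the first input's data to PCG dynamic mesh data and stops if that fails.
; It then replaces the mesh's materials with the single Material variable and outputs that same mesh data, with no geometry edits.
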(fn ExecutewithContext
  (params (InContext :type PCG%20Context%20Structure%20%28by%20ref%29) (Input :type PCG%20Data%20Collection%20Structure%20%28by%20ref%29))
  (Utilities|FlowControl|Sequence
    (:then_0
      (bind _returnvalue (Class|PCGDataFunctionLibrary|GetInputs Input))
      (bind _aspcgdynamic_mesh_data (Utilities|Casting|CastToPCGDynamicMeshData (.Data (Utilities|Struct|BreakPCGTaggedData (Utilities|Array|Get(acopy) _returnvalue)))))
      (LocalVariables|SetPCGDynamicMesh _aspcgdynamic_mesh_data))
    (:then_2
      (Class|PCGDynamicMeshData|SetMaterials (LocalVariables|GetPCGDynamicMesh) (Utilities|Array|MakeArray (Variables|Default|GetMaterial)))
      (return (Utilities|Struct|MakePCGDataCollection (Utilities|Array|MakeArray (Utilities|Struct|MakePCGTaggedData (LocalVariables|GetPCGDynamicMesh) 0 "None")))))))