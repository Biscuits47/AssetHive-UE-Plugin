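; PCG snow tool actor that generates snow meshes on reference actors and bakes them to static mesh assets.
; Construction adds a box or sphere volume, feeds scatter mode, scale-based remesh resolution and active state to the PCG graph, and syncs reference tags across all instances.
; Save triggers export to a PCGMesh folder beside the level under a random name.
; Place spawns the saved mesh, attaches it to a lone reference and deactivates PCG.
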(fn ConstructionScript
  (CallFunction|CreateSnow))

(fn CreateSnow
  (bind _pcg (Variables|Default|GetPCG))
  (bind _pcg_2 (Variables|Default|GetPCG))
  (bind _graphinstance (Variables|/Script/PCG.PCGComponent|GetGraphInstance _pcg))
  (bind _graphinstance_2 (Variables|/Script/PCG.PCGComponent|GetGraphInstance _pcg_2))
  (if (Utilities|Enum|Equal(Enum) (Variables|01-Global|GetVoulme%20Sphere) "NewEnumerator0")
    (AddComponent|AddBoxComponent false)
    (else
      (AddComponent|AddSphereComponent false)))
  (Class|PCGGraphParametersHelpers|SetInt32Parameter _graphinstance_2 "ScatterMode" (Utilities|Select :Index (Variables|01-Global|GetMode) :NewEnumerator0 0 :NewEnumerator1 1))
  (Class|PCGGraphParametersHelpers|SetInt32Parameter _graphinstance_2 "RemeshRes" (Math|Float|Truncate (* (Math|Vector|DotProduct (Math|Vector|VectorGetAbs (Transformation|GetActorScale3D self)) "0.333000,0.333000,0.333000") (Variables|02-Sphere|GetRemesh%20Resloution))))
  (if (Variables|01-Global|GetActive)
    (Effects|Components|ParticleSystem|SetBoolParameter _graphinstance "Active" true)
    (Variables|/Script/PCG.PCGComponent|SetbActivated _pcg true)
    (else
      (Effects|Components|ParticleSystem|SetBoolParameter _graphinstance "Active" false)
      (Variables|/Script/PCG.PCGComponent|SetbActivated _pcg false)))
  (for _array_element (Variables|01-Global|GetRerfenceMesh)
    (if (not (Actor|ActorHasTag _array_element "RerfenceMesh"))
      (Utilities|Array|Add (Variables|/Script/Engine.Actor|GetTags _array_element) "RerfenceMesh")
      (Variables|/Script/Engine.Actor|SetTags _array_element (Variables|/Script/Engine.Actor|GetTags _array_element))))
  (CallFunction|RemoveExtraTags))

(fn 01-SavetoAsset
  (bind _returnvalue (Class|Actor|GetLevel))
  (bind _pcg (Variables|Default|GetPCG))
  (bind _returnvalue_2 (Class|KismetSystemLibrary|GetPathName _returnvalue))
  (bind _graphinstance (Variables|/Script/PCG.PCGComponent|GetGraphInstance _pcg))
  (bind _returnvalue_3 (Utilities|String|Len _returnvalue_2))
  (bind _returnvalue_4 (Utilities|String|Reverse _returnvalue_2))
  (bind _returnvalue_5 (Utilities|String|FindSubstring _returnvalue_4 "/"))
  (bind _returnvalue_6 (- _returnvalue_3 _returnvalue_5))
  (bind _returnvalue_7 (Utilities|String|Left _returnvalue_2 _returnvalue_6))
  (bind _returnvalue_8 (Utilities|String|Append _returnvalue_7 "PCGMesh" "/"))
  (bind _name (CallFunction|GetRandomName 5))
  (Variables|BakeMesh|SetMesh%20Name (Utilities|String|Append "SM_Snow" "_" _name))
  (Variables|BakeMesh|SetMesh%20Path _returnvalue_8)
  (bind _asset_exists (CallFunction|ValidateAssetsExists (Utilities|String|Append _returnvalue_8 (Utilities|String|Append "SM_Snow" "_" _name) "." (Utilities|String|Append "SM_Snow" "_" _name) " ")))
  (Class|PCGGraphParametersHelpers|SetStringParameter _graphinstance "MeshName" (Variables|BakeMesh|GetMesh%20Name))
  (Class|PCGGraphParametersHelpers|SetStringParameter _graphinstance "MeshPath" (Variables|BakeMesh|GetMesh%20Path))
  (if (not _asset_exists)
    (Effects|Components|ParticleSystem|SetBoolParameter _graphinstance "Savemesh" true)))

(fn 02-PlaceinLevel
  (bind _mesh_name (Variables|BakeMesh|GetMesh%20Name))
  (bind _pcg (Variables|Default|GetPCG))
  (bind _rerfencemesh (Variables|01-Global|GetRerfenceMesh))
  (bind _graphinstance (Variables|/Script/PCG.PCGComponent|GetGraphInstance _pcg))
  (bind _asset_exists (CallFunction|ValidateAssetsandPath))
  (if _asset_exists
    (bind _returnvalue (Game|SpawnActorfromClass "/Script/Engine.StaticMeshActor" (Math|Conversions|ToTransform(Vector) (.location (Transformation|GetActorTransform))) "Undefined" "MultiplyWithRoot" 0 0))
    (bind _returnvalue_2 (Utilities|LoadAssetBlocking (Class|KismetSystemLibrary|ToSoftObjRef(SoftObjPath) (Utilities|MakeSoftObjectPath (Utilities|String|Append (Variables|BakeMesh|GetMesh%20Path) _mesh_name "." _mesh_name)))))
    (bind _asstatic_mesh (Utilities|Casting|CastToStaticMesh _returnvalue_2))
    (Components|StaticMesh|SetStaticMesh (Variables|/Script/Engine.StaticMeshActor|GetStaticMeshComponent _returnvalue) _asstatic_mesh)
    (Variables|/Script/Engine.ActorComponent|SetComponentTags (Variables|/Script/Engine.StaticMeshActor|GetStaticMeshComponent _returnvalue) (Utilities|Array|MakeArray "PCGMesh"))
    (if (> (Utilities|Array|Length _rerfencemesh) 1)
      _
      (else
        (Transformation|AttachActorToActor _returnvalue (Utilities|Array|Get(acopy) _rerfencemesh) "None" "KeepWorld" "KeepWorld" "KeepWorld" true)))
    (Effects|Components|ParticleSystem|SetBoolParameter _graphinstance "Savemesh" false)
    (Effects|Components|ParticleSystem|SetBoolParameter _graphinstance "Active" false)
    (Variables|01-Global|SetActive false)
    (else
      (Development|PrintString "未生成资产！" true true "(R=1.000000,G=0.039770,B=0.009923,A=1.000000)" 1e+01))))

(fn ReGenerate
  (bind _pcg (Variables|Default|GetPCG))
  (Class|PCGComponent|CleanupLocal _pcg true false)
  (Class|PCGComponent|GenerateLocal _pcg true))

(fn ValidateAssetsandPath
  (bind _mesh_name (Variables|BakeMesh|GetMesh%20Name))
  (bind _returnvalue (Class|AssetRegistry|GetAssetbyObjectPath (Class|AssetRegistryHelpers|GetAssetRegistry) (Utilities|String|StringToName (Utilities|String|Append (Variables|BakeMesh|GetMesh%20Path) _mesh_name "." _mesh_name)) false))
  (return (Utilities|IsValid (Class|AssetRegistryHelpers|GetAsset _returnvalue))))

(fn RemoveExtraTags
  (Utilities|Array|Clear (Variables|DontTouch|GetAll%20Rerfence%20Mesh))
  (bind _outactors (Actor|GetAllActorsOfClass "BP_PCG_Snow_C"))
  (for _array_element _outactors
    (Utilities|Array|AppendArray (Variables|DontTouch|GetAll%20Rerfence%20Mesh) (Variables|BP_PCG_Snow_C|GetRerfenceMesh _array_element)))
  (Utilities|Array|Clear (Variables|DontTouch|GetRerfence%20Actors))
  (bind _outactors_2 (Actor|GetAllActorswithTag "RerfenceMesh"))
  (Variables|DontTouch|SetRerfence%20Actors _outactors_2)
  (LocalVariables|SetRemove%20Count 0)
  (for (_array_element_2 _array_index) _outactors_2
    (Utilities|Casting|CastToStaticMeshActor _array_element_2
      (:then
        (bind _array_element_3 (Utilities|Array|ForEachLoopwithBreak (Variables|DontTouch|GetAll%20Rerfence%20Mesh) :!label _label)
          (:LoopBody
            (if (== _array_element_3 _array_element_2)
              (Utilities|Array|RemoveIndex (Variables|DontTouch|GetRerfence%20Actors) (- _array_index (LocalVariables|GetRemove%20Count)))
              (Math|Integer|IncrementInt (LocalVariables|GetRemove%20Count)
                (:%20%20
                  (goto _label Break)))))))
      (:CastFailed
        (Utilities|Array|RemoveIndex (Variables|DontTouch|GetRerfence%20Actors) (- _array_index (LocalVariables|GetRemove%20Count)))
        (Math|Integer|IncrementInt (LocalVariables|GetRemove%20Count)))))
  (for _array_element_4 (Variables|DontTouch|GetRerfence%20Actors)
    (Utilities|Array|Clear (Variables|DontTouch|GetNew%20Tag))
    (for _array_element_5 (Variables|/Script/Engine.Actor|GetTags _array_element_4)
      (if (not (== _array_element_5 "RerfenceMesh"))
        (Utilities|Array|Add (Variables|DontTouch|GetNew%20Tag) _array_element_5)))
    (Variables|/Script/Engine.Actor|SetTags _array_element_4 (Variables|DontTouch|GetNew%20Tag))))