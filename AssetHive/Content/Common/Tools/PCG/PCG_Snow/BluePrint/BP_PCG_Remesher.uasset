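; A custom PCG Blueprint node in the snow tool that remeshes incoming dynamic mesh data using Geometry Script.
; It edits the first input mesh through SDF-grid morphology driven by thickness and cell resolution, then iterative smoothing and box-projected UVs.
; An optional simplify pass reduces triangles to a percentage of the current count.
; The mesh gets a single configurable material and is returned as the node's output.
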(fn ExecutewithContext
  (params (InContext :type PCG%20Context%20Structure%20%28by%20ref%29) (Input :type PCG%20Data%20Collection%20Structure%20%28by%20ref%29))
  (Utilities|FlowControl|Sequence
    (:then_0
      (bind _returnvalue (Class|PCGDataFunctionLibrary|GetInputs Input))
      (bind _aspcgdynamic_mesh_data (Utilities|Casting|CastToPCGDynamicMeshData (.Data (Utilities|Struct|BreakPCGTaggedData (Utilities|Array|Get(acopy) _returnvalue)))))
      (bind _output_get (LocalVariables|SetPCGDynamicMesh _aspcgdynamic_mesh_data)))
    (:then_1
      (bind _returnvalue_2 (Class|GeometryScriptLibraryMeshVoxelFunctions|ApplyMeshMorphology (Variables|/Script/PCGGeometryScriptInterop.PCGDynamicMeshData|GetDynamicMesh (LocalVariables|GetPCGDynamicMesh)) (Utilities|Struct|MakeGeometryScriptMorphologyOptions (Utilities|Struct|MakeGeometryScript3DGridParameters "GridResolution" 0.5 (Variables|Default|GetCell%20Res)) false "(SizeMethod=GridResolution,GridCellSize=0.500000,GridResolution=64)" "Dilate" (Variables|Default|GetThickness)) 0))
      (bind _returnvalue_3 (Class|GeometryScriptLibraryMeshDeformFunctions|ApplyIterativeSmoothingtoMesh :TargetMesh _returnvalue_2 :Options (Utilities|Struct|MakeGeometryScriptIterativeMeshSmoothingOptions (Variables|Default|GetSmooth%20Lterations) (Variables|Default|GetSmooth%20Strength) "FullMeshSelection") :Debug 0))
      (bind _returnvalue_4 (Class|GeometryScriptLibraryMeshUVFunctions|SetMeshUVsfromBoxProjection :TargetMesh _returnvalue_3 :BoxTransform (Math|Transform|MakeTransform "0, 0, 0" "0, 0, 0" "500.000000,500.000000,500.000000") :Debug 0))
      (if (Variables|Default|GetUse%20Simplify)
        (bind _returnvalue_5 (Class|GeometryScriptLibraryMeshSimplifyFunctions|ApplySimplifytoTriangleCount _returnvalue_4 (Math|Float|Truncate (* (Math|Float|Clamp(Float) (/ (Variables|Default|GetSimplify%20Pecentage) 1e+02)) (Class|DynamicMesh|GetTriangleCount _returnvalue_4))) (Utilities|Struct|MakeGeometryScriptSimplifyMeshOptions "AttributeAware" true true true false false true) 0))
        (Variables|Default|SetCurrent%20Triangle%20Count (Class|DynamicMesh|GetTriangleCount _returnvalue_5))))
    (:then_2
      (Class|PCGDynamicMeshData|SetMaterials (LocalVariables|GetPCGDynamicMesh) (Utilities|Array|MakeArray (Variables|Default|GetMaterial)))
      (return (Utilities|Struct|MakePCGDataCollection (Utilities|Array|MakeArray (Utilities|Struct|MakePCGTaggedData (LocalVariables|GetPCGDynamicMesh) 0 "None")))))))