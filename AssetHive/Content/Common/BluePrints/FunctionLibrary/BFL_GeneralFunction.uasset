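; General-purpose Blueprint function library with helpers for random names and asset paths.
; GetRandomName builds a string of a given length from random picks in a letters-and-numbers array.
; ValidateAssetsExists looks up an object path in the Asset Registry, including in-memory assets, and checks that the resolved asset is valid.
; GetSingleAssetPath trims the trailing object name and its separator from an object's path name, leaving the package path.
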(fn GetRandomName
  (params (Length :type Integer))
  (LocalVariables|SetRandomName "")
  (for _index (range 0 (- Length 1))
    (LocalVariables|SetRandomName (Utilities|String|Append (LocalVariables|GetRandomName) (Utilities|Array|Get(acopy) (LocalVariables|GetLettersArray%20and%20Number) (Math|Random|RandomIntegerinRange 0 (- (Utilities|Array|Length (LocalVariables|GetLettersArray%20and%20Number)) 1))))))
  (return (LocalVariables|GetRandomName)))

(fn ValidateAssetsExists
  (params (Path :type String))
  (bind _returnvalue (Class|AssetRegistry|GetAssetbyObjectPath (Class|AssetRegistryHelpers|GetAssetRegistry) (Utilities|String|StringToName Path) false))
  (return (Utilities|IsValid (Class|AssetRegistryHelpers|GetAsset _returnvalue))))

(fn GetSingleAssetPath
  (params (Object :type Object%20Object%20Reference))
  (bind _returnvalue (Class|KismetSystemLibrary|GetPathName Object))
  (return (Utilities|String|Left _returnvalue (- (Utilities|String|Len _returnvalue) (+ (Utilities|String|Len (Utilities|GetObjectName Object)) 1)))))